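; AI enemy that chases or reacts to the player through a blackboard and either hurts the player or dies on contact.
; AI perception writes the sensed actor to the Seenplayer blackboard key and clears it when sensing fails.
; Sphere overlap removes player health through BPHealthSystem, unless the player is attacking.
; In that case the enemy's mesh simulates physics, and after a delay it spawns a coin and destroys itself.
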(event OnTargetPerceptionUpdated(AIPerception)
  (params (Actor :type Actor%20Object%20Reference) (Stimulus :type AI%20Stimulus%20Structure))
  (bind _returnvalue (Pawn|GetController))
  (bind _returnvalue_2 (Utilities|Name|MakeLiteralName "Seenplayer"))
  (bind _returnvalue_3 (AI|GetBlackboard _returnvalue))
  (if (.bsuccessfullysensed Stimulus)
    (AI|Components|Blackboard|SetValueasObject _returnvalue_3 _returnvalue_2 Actor)
    (else
      (AI|Components|Blackboard|SetValueasObject _returnvalue_3 _returnvalue_2 0))))

(event OnComponentBeginOverlap(Sphere)
  (params (OverlappedComponent :type Primitive%20Component%20Object%20Reference) (OtherActor :type Actor%20Object%20Reference) (OtherComp :type Primitive%20Component%20Object%20Reference) (OtherBodyIndex :type Integer) (bFromSweep :type Boolean) (SweepResult :type Hit%20Result%20Structure%20%28by%20ref%29))
  (bind _returnvalue (Transformation|GetActorLocation))
  (if (== OtherActor (Variables|Default|GetPlayer))
    (if (Variables|/Game/ThirdPerson/Blueprints/BP_ThirdPersonCharacter.BP_ThirdPersonCharacter_C|GetisAttacking (Variables|Default|GetPlayer))
      (Physics|SetSimulatePhysics (Variables|Character|GetMesh) true)
      (Physics|AddForce (Variables|Character|GetMesh) "-100.000000,0.000000,0.000000" "None" false)
      (Utilities|FlowControl|Delay 5.0)
      (Game|SpawnActorfromClass "/Game/MoraBermejoSebastian/BP_EnemyCoin.BP_EnemyCoin_C" (Math|Transform|MakeTransform (Math|Vector|MakeVector (.x _returnvalue) (.y _returnvalue) 5.0) "0, 0, 0" "1.000000,1.000000,1.000000") "Undefined" "MultiplyWithRoot" 0 0)
      (Actor|DestroyActor)
      (else
        (Default|RemoveHealth (Variables|Default|GetPlayerSystem) (Variables|Default|GetDamage) true)))))

(event EventBeginPlay
  (bind _output_get (Variables|Default|SetOriginPos (Transformation|GetActorLocation)))
  (Transformation|SetActorLocation _output_get false false)
  ;[0.09835 0.6771 0.6569] Get a reference to the health system of the player
  (bind _outactors (Actor|GetAllActorsOfClass "/Game/ThirdPerson/Blueprints/BP_ThirdPersonCharacter.BP_ThirdPersonCharacter_C"))
  (Variables|Default|SetPlayer (Utilities|Array|Get(acopy) _outactors))
  (Variables|Default|SetPlayerSystem (Variables|/Game/ThirdPerson/Blueprints/BP_ThirdPersonCharacter.BP_ThirdPersonCharacter_C|GetBP_HealthSystem (Utilities|Array|Get(acopy) _outactors))))

(fn ConstructionScript)