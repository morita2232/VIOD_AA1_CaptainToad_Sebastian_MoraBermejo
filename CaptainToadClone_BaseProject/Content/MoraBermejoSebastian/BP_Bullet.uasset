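; Projectile Blueprint that damages the player's health.
; On BeginPlay it caches the health system of the first BP_ThirdPersonCharacter found.
; Tick sweeps it along local X by Speed plus a small delta-time-scaled term, and a 10-second delay destroys it.
; A capsule overlap with any component not simulating physics removes Damage from that cached health system and destroys the bullet, without checking what was hit.
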(event OnComponentBeginOverlap(Capsule)
  (params (OverlappedComponent :type Primitive%20Component%20Object%20Reference) (OtherActor :type Actor%20Object%20Reference) (OtherComp :type Primitive%20Component%20Object%20Reference) (OtherBodyIndex :type Integer) (bFromSweep :type Boolean) (SweepResult :type Hit%20Result%20Structure%20%28by%20ref%29))
  ;[0.09835 0.6771 0.6569] Check if bullet has hit the player
  (if (not (Physics|IsSimulatingPhysics OtherComp "None"))
    ;[0.09835 0.6771 0.6569] Remove health from the player and destroy bullet
    (Default|RemoveHealth (Variables|Default|GetPlayerSystem) (Variables|Default|GetDamage))
    (Actor|DestroyActor)))

(event EventBeginPlay
  ;[0.09835 0.6771 0.6569] Get a reference to the health system of the player
  (bind _outactors (Actor|GetAllActorsOfClass "/Game/ThirdPerson/Blueprints/BP_ThirdPersonCharacter.BP_ThirdPersonCharacter_C"))
  (Variables|Default|SetPlayerSystem (Variables|/Game/ThirdPerson/Blueprints/BP_ThirdPersonCharacter.BP_ThirdPersonCharacter_C|GetBP_HealthSystem (Utilities|Array|Get(acopy) _outactors))))

(event EventTick
  (params (DeltaSeconds :type Float%20%28single-precision%29))
  ;[0.09835 0.6771 0.6569] Move the bullet
  (Transformation|AddActorLocalOffset (Math|Vector|MakeVector (+ (Variables|Default|GetSpeed) (* (.x (Math|Vector|GetRightVector (Variables|Default|GetStaticMesh))) DeltaSeconds)) 0.0 0.0) true false)
  ;[0.09835 0.6771 0.6569] Destroy fter 10 seconds if it hasnt hit anything
  (Utilities|FlowControl|Delay 1e+01)
  (Actor|DestroyActor))

(fn ConstructionScript
  (|CallParentFunction))