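; BP_Button is a weight-sensitive button that reacts to Box actors entering its trigger.
; It saves StaticMesh1's location at BeginPlay, then on overlap stops an entering box's velocity and sweeps it to that point.
; If the box's mass exceeds WeightLimit it calls OFF.
; Any end overlap calls ON, with no class or weight check.
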(event OnComponentBeginOverlap(Box)
  (params (OverlappedComponent :type Primitive%20Component%20Object%20Reference) (OtherActor :type Actor%20Object%20Reference) (OtherComp :type Primitive%20Component%20Object%20Reference) (OtherBodyIndex :type Integer) (bFromSweep :type Boolean) (SweepResult :type Hit%20Result%20Structure%20%28by%20ref%29))
  ;[0.09835 0.6771 0.6569] Check if the object entering the collider is a "box"
  (bind _asbox (Utilities|Casting|CastToBox OtherActor))
  (if (== (Utilities|GetClass OtherActor) "/Game/MoraBermejoSebastian/Box.Box_C")
    ;[0.09835 0.6771 0.6569] Stop the "box" from moving before being set in the point we tell it to
    (Physics|SetPhysicsLinearVelocity (Variables|/Game/MoraBermejoSebastian/Box.Box_C|GetStaticMesh _asbox) "0, 0, 0" false "None")
    ;[0.09835 0.6771 0.6569] Set the "box" in the point we saved earlier
    (Transformation|SetWorldLocation (Variables|/Game/MoraBermejoSebastian/Box.Box_C|GetStaticMesh _asbox) (Variables|Default|GetLocaion) true false)
    ;[0.09835 0.6771 0.6569] Check if the mass of the object can activate the button
    (if (< (Variables|Default|GetweightLimit) (Variables|/Game/MoraBermejoSebastian/Box.Box_C|GetMass _asbox))
      (CallFunction|OFF))))

(event OnComponentEndOverlap(Box)
  (params (OverlappedComponent :type Primitive%20Component%20Object%20Reference) (OtherActor :type Actor%20Object%20Reference) (OtherComp :type Primitive%20Component%20Object%20Reference) (OtherBodyIndex :type Integer))
  ;[0.09835 0.6771 0.6569] Turn off the button
  (CallFunction|ON))

(event EventBeginPlay
  ;[0.09835 0.6771 0.6569] Get the position of the point where objects will be put in
  (Variables|Default|SetLocaion (Transformation|GetWorldLocation (Variables|Default|GetStaticMesh1))))

(fn ConstructionScript
  (|CallParentFunction))