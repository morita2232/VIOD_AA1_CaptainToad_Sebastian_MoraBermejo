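; BP_CrystalCounter tracks how many crystals the player has collected and reports when the goal is reached.
; The Add event increments the Crystals count and calls Check, which compares it against MaxCrystals.
; Check prints the collected and remaining counts while below the maximum, and a win message otherwise.
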(event Custom|Add
  ;[0.09835 0.6771 0.6569] Adding 1 crystal to the count and checking if we have all of them
  (Variables|Default|SetCrystals (+ (Variables|Default|GetCrystals) 1))
  (CallFunction|Check))

(event Custom|Check
  ;[0.09835 0.6771 0.6569] Check if the player has the 5 crystals
  (if (< (Variables|Default|GetCrystals) (Variables|Default|GetMaxCrystals))
    ;[0.09835 0.6771 0.6569] How many crystals the player has collected
    (Development|PrintString (Utilities|String|Append "You have " (Utilities|String|ToString(Integer) (Variables|Default|GetCrystals)) " crystal/s!"))
    ;[0.09835 0.6771 0.6569] How many crystal the player has left to collect
    (Development|PrintString (Utilities|String|Append "Only " (Utilities|String|ToString(Integer) (- (Variables|Default|GetMaxCrystals) (Variables|Default|GetCrystals))) " crystal/s to go!"))
    (else
      ;[0.09835 0.6771 0.6569] Win message
      (Development|PrintString "YOU WIN"))))

(fn ConstructionScript)