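; Elevator actor that moves between its start position and an offset destination when switched on or off by a lever.
; On BeginPlay it stores the mesh's world location and registers itself in the Actors list of its child-actor BP_Lever.
; SwitchON plays the Move timeline from the start and SwitchOFF reverses it from the end, lerping the actor's location between PosA and PosA + PosB without sweeping.
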(event EventBeginPlay
  ;[0.09835 0.6771 0.6569] Getting the start position of the elevator
  (Variables|Default|SetposA (Transformation|GetWorldLocation (Variables|Default|GetStaticMesh)))
  ;[0.09835 0.6771 0.6569] Adding the elevator to the lever who is a child actor in this object
  (bind _asbp_lever (Utilities|Casting|CastToBP_Lever (Variables|/Script/Engine.ChildActorComponent|GetChildActor (Variables|Default|GetChildActor))))
  (Utilities|Array|Add (Variables|/Game/MoraBermejoSebastian/BP_InteractableObject.BP_InteractableObject_C|GetActors _asbp_lever) self))

(event EventSwitchON
  (bind _posa (Variables|Default|GetposA))
  ;[0.09835 0.6771 0.6569] Receives the signal ON or OFF, according to which on it receives the timeline plays normally or reversed, then we set the location according to the timeline and the lerp from point A and B
  (bind _newtrack_0 (Timeline|Move PlayFromStart)
    (:Update
      (Transformation|SetActorLocation (Math|Vector|Lerp(Vector) _posa (+ _posa (Variables|Default|GetposB)) _newtrack_0) false false))
    (:Finished
      (Timeline|Move Stop))))

(event EventSwitchOFF
  (bind _posa (Variables|Default|GetposA))
  ;[0.09835 0.6771 0.6569] Receives the signal ON or OFF, according to which on it receives the timeline plays normally or reversed, then we set the location according to the timeline and the lerp from point A and B
  (bind _newtrack_0 (Timeline|Move ReverseFromEnd)
    (:Update
      (Transformation|SetActorLocation (Math|Vector|Lerp(Vector) _posa (+ _posa (Variables|Default|GetposB)) _newtrack_0) false false))
    (:Finished
      (Timeline|Move Stop))))

(fn ConstructionScript
  (|CallParentFunction))