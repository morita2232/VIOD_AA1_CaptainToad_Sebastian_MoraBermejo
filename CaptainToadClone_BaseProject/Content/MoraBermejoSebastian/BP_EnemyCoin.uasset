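; BP_EnemyCoin is a coin pickup that adds its value to the player's coin count on the HUD.
; After a short delay at BeginPlay, it caches the third-person character and the coins and crystals widget found inside the first WBP_HUD, with debug prints for validity.
; When that player overlaps its sphere, it calls UpdateCoins on the widget with its Value and destroys itself.
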(event OnComponentBeginOverlap(Sphere)
  (params (OverlappedComponent :type Primitive%20Component%20Object%20Reference) (OtherActor :type Actor%20Object%20Reference) (OtherComp :type Primitive%20Component%20Object%20Reference) (OtherBodyIndex :type Integer) (bFromSweep :type Boolean) (SweepResult :type Hit%20Result%20Structure%20%28by%20ref%29))
  (if (== OtherActor (Variables|Default|GetPlayer))
    (Default|UpdateCoins (Variables|Default|GetWBP%20Crystals%20and%20Coins) (Variables|Default|GetValue))
    (Actor|DestroyActor)))

(event EventBeginPlay
  (Utilities|FlowControl|Delay 0.2)
  (Development|PrintString "coin spawned")
  (bind _returnvalue (Actor|GetActorOfClass "/Game/ThirdPerson/Blueprints/BP_ThirdPersonCharacter.BP_ThirdPersonCharacter_C"))
  (Variables|Default|SetPlayer _returnvalue)
  (bind _foundwidgets (Widget|GetAllWidgetsOfClass "/Game/MoraBermejoSebastian/WBP_HUD.WBP_HUD_C" true))
  (bind _output_get (Variables|Default|SetHUD (Utilities|Array|Get(acopy) _foundwidgets)))
  (Utilities|IsValid _output_get
    (:Is%20Valid
      (bind _output_get_2 (Variables|Default|SetWBP%20Crystals%20and%20Coins (Variables|/Game/MoraBermejoSebastian/WBP_HUD.WBP_HUD_C|GetWBP_CrystalsAndCoins _output_get)))
      (Utilities|IsValid _output_get_2
        (:Is%20Valid
          (Development|PrintString "VALID"))
        (:Is%20Not%20Valid
          (Development|PrintString "NOT VALID"))))
    (:Is%20Not%20Valid
      (Development|PrintString "NOT VALID 1"))))

(fn ConstructionScript)