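; Health system that tracks current life for its owner and handles healing, damage and death.
; CurrentLife starts at MaxLife on BeginPlay, and AddHealth and RemoveHealth keep it clamped between zero and that maximum.
; Both functions broadcast the requested amount, then the new health, through event dispatchers.
; Death prints a message and opens the level passed by name; nothing here calls it when life reaches zero.
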(event EventBeginPlay
  (Variables|Default|SetCurrentLife (Variables|Default|GetMaxLife)))

(fn AddHealth
  (params (Amount :type Float%20%28double-precision%29) (Heal :type Boolean))
  ;[0.09835 0.6771 0.6569] Receives an amount to health to add to the current one
  (bind _output_get (Variables|Default|SetCurrentLife (Math|Float|Clamp(Float) (+ (Variables|Default|GetCurrentLife) Amount) 0.0 (Variables|Default|GetMaxLife))))
  ;[0.09835 0.6771 0.6569] Notify we healed and the health has changed
  (Default|CallOnHealthHealed Amount Heal)
  (Default|CallOnHealthChanged _output_get Heal))

(fn RemoveHealth
  (params (Amount :type Float%20%28double-precision%29) (Damaged :type Boolean))
  ;[0.09835 0.6771 0.6569] Receives an ammount of health to be removed from the current one
  (bind _output_get (Variables|Default|SetCurrentLife (Math|Float|Clamp(Float) (- (Variables|Default|GetCurrentLife) Amount) 0.0 (Variables|Default|GetMaxLife))))
  ;[0.09835 0.6771 0.6569] Notify we have lost health and that health has changed
  (Default|CallOnHealthDamaged Amount Damaged)
  (Default|CallOnHealthChanged _output_get Damaged))

(fn Death
  (params (LevelName :type String))
  ;[0.09835 0.6771 0.6569] Notifies the player they have died and reloads the level according to the name it receives
  (Development|PrintString "YOU DIED" true true "(R=0.000000,G=0.660000,B=1.000000,A=1.000000)" 1e+01)
  (Game|OpenLevel(byName) (Utilities|String|StringToName LevelName)))