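; BP_Heart is a health pickup that adds health to the player when touched.
; On BeginPlay it caches the BPHealthSystem of the first BP_ThirdPersonCharacter found in the level.
; When any actor without the "Enemy" tag overlaps its Sphere, it adds its Heal amount to that cached health system, whichever actor triggered it, then destroys itself.
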(event OnComponentBeginOverlap(Sphere)
  (params (OverlappedComponent :type Primitive%20Component%20Object%20Reference) (OtherActor :type Actor%20Object%20Reference) (OtherComp :type Primitive%20Component%20Object%20Reference) (OtherBodyIndex :type Integer) (bFromSweep :type Boolean) (SweepResult :type Hit%20Result%20Structure%20%28by%20ref%29))
  (if (not (Actor|ActorHasTag OtherActor "Enemy"))
    (Default|AddHealth (Variables|Default|GetBP%20Health%20System) (Variables|Default|GetHeal) false)
    (Actor|DestroyActor)))

(event EventBeginPlay
  ;[0.09835 0.6771 0.6569] Get a reference to the health system of the player
  (bind _outactors (Actor|GetAllActorsOfClass "/Game/ThirdPerson/Blueprints/BP_ThirdPersonCharacter.BP_ThirdPersonCharacter_C"))
  (Variables|Default|SetBP%20Health%20System (Variables|/Game/ThirdPerson/Blueprints/BP_ThirdPersonCharacter.BP_ThirdPersonCharacter_C|GetBP_HealthSystem (Utilities|Array|Get(acopy) _outactors))))

(fn ConstructionScript
  (|CallParentFunction))