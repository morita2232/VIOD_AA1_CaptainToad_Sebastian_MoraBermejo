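; BP_InteractableObject is an actor that relays on and off signals to an array of target actors.
; Its ON and OFF functions loop over that array and send SwitchONMessage or SwitchOFFMessage to each actor implementing the I_SignalReceiver interface, so targets need no specific class.
; The file has no live trigger for either function, as the only ON call in the event graph never runs.
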(fn ConstructionScript)

(fn ON
  ;[0.09835 0.6771 0.6569] Looks at the whole array of actors
  (for _array_element (Variables|Default|GetActors)
    ;[0.09835 0.6771 0.6569] Check if it implements the neccesary interface, if it does, sends the ON signal
    (if (Utilities|DoesObjectImplementInterface _array_element "/Game/MoraBermejoSebastian/I_SignalReceiver.I_SignalReceiver_C")
      (Class|ISignalReceiver|SwitchON(Message) _array_element))))

(fn OFF
  ;[0.09835 0.6771 0.6569] Looks at the whole array of actors
  (for _array_element (Variables|Default|GetActors)
    ;[0.09835 0.6771 0.6569] Checks if it implements the neccesary interface, if it does, sends the OFF signal
    (if (Utilities|DoesObjectImplementInterface _array_element "/Game/MoraBermejoSebastian/I_SignalReceiver.I_SignalReceiver_C")
      (Class|ISignalReceiver|SwitchOFF(Message) _array_element))))