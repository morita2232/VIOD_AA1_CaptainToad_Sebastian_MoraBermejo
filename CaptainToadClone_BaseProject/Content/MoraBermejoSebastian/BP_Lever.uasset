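; BP_Lever is an interactable lever that plays a switch sound and alternates between ON and OFF signals.
; INTERACT uses a FlipFlop to call ON or OFF, sets the player character's Onoff flag, then calls UPDATE.
; UPDATE picks a toggle animation from that flag, which is cached from the first BP_ThirdPersonCharacter at BeginPlay.
; Both FlipFlop branches set Onoff to true, so interaction always selects the toggleoff animation.
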(event Custom|INTERACT
  ;[0.09835 0.6771 0.6569] Tells the switch which signal to send
  (Audio|SpawnSoundAttached "/Game/CaptainToadSFX/SFX_Switch_Cue.SFX_Switch_Cue" (Variables|/Script/Engine.Character|GetMesh (Variables|Default|GetCharacter)) "None" "0, 0, 0" "0, 0, 0" "KeepWorldPosition" false 1.0 1.0 0.0 0 0)
  (Utilities|FlowControl|FlipFlop
    (:A
      (CallFunction|ON)
      (Variables|/Game/ThirdPerson/Blueprints/BP_ThirdPersonCharacter.BP_ThirdPersonCharacter_C|Seton/off (Variables|Default|GetCharacter) true))
    (:B
      (CallFunction|OFF)
      (Variables|/Game/ThirdPerson/Blueprints/BP_ThirdPersonCharacter.BP_ThirdPersonCharacter_C|Seton/off (Variables|Default|GetCharacter) true)))
  (CallFunction|UPDATE))

(event Custom|UPDATE
  ;[0.09835 0.6771 0.6569] Checks if the switch is on or off
  (if (Variables|/Game/ThirdPerson/Blueprints/BP_ThirdPersonCharacter.BP_ThirdPersonCharacter_C|Geton/off (Variables|Default|GetCharacter))
    ;[0.09835 0.6771 0.6569] It plays the according animation to the state of the lever
    (Components|Animation|PlayAnimation (Variables|Default|GetSkeletalMesh) "/Game/Assets/lever_Anim_toggle-off.lever_Anim_toggle-off" false)
    (else
      (Components|Animation|PlayAnimation (Variables|Default|GetSkeletalMesh) "/Game/Assets/lever_Anim_toggle-on.lever_Anim_toggle-on" false))))

(event EventBeginPlay
  ;[0.09835 0.6771 0.6569] Gets the reference to the player
  (bind _outactors (Actor|GetAllActorsOfClass "/Game/ThirdPerson/Blueprints/BP_ThirdPersonCharacter.BP_ThirdPersonCharacter_C"))
  (Variables|Default|SetCharacter (Utilities|Array|Get(acopy) _outactors)))

(fn ConstructionScript
  (|CallParentFunction))