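; BP_Lock is a lock actor that opens when the key touches it.
; On BeginPlay it caches the first BP_Key found in the level, so it responds only to that single instance.
; When that key overlaps its Box, the lock calls OFF to signal the unlocked state, clears the key's IsPicked flag and destroys both actors.
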(event OnComponentBeginOverlap(Box)
  (params (OverlappedComponent :type Primitive%20Component%20Object%20Reference) (OtherActor :type Actor%20Object%20Reference) (OtherComp :type Primitive%20Component%20Object%20Reference) (OtherBodyIndex :type Integer) (bFromSweep :type Boolean) (SweepResult :type Hit%20Result%20Structure%20%28by%20ref%29))
  ;[0.09835 0.6771 0.6569] Checks if the object it has overlapped with is a key
  (if (== OtherActor (Variables|Default|GetKey))
    ;[0.09835 0.6771 0.6569] If it is a key, it send the off (unlocked) signal and destroys both actors
    (CallFunction|OFF)
    (Variables|/Game/MoraBermejoSebastian/BP_PickableObject.BP_PickableObject_C|SetIsPicked (Variables|Default|GetKey) false)
    (Actor|DestroyActor)
    (Actor|DestroyActor OtherActor)))

(event EventBeginPlay
  ;[0.09835 0.6771 0.6569] Get reference to the key
  (bind _returnvalue (Actor|GetActorOfClass "/Game/MoraBermejoSebastian/BP_Key.BP_Key_C"))
  (Variables|Default|SetKey _returnvalue))

(fn ConstructionScript
  (|CallParentFunction))