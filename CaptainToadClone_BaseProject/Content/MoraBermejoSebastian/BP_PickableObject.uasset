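; Pickable physics object that the third-person character can grab and throw.
; On BeginPlay it caches its static mesh and the first BP_ThirdPersonCharacter found, then simulates physics with gravity off until thrown.
; PickUp grabs the given component through the passed physics handle and sets IsPicked.
; Drop releases it and always calls Throw, which enables gravity, adds a velocity-change impulse along the character's forward vector and clears IsPicked.
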(event EventBeginPlay
  (Variables|Default|SetMyMesh (Actor|GetComponentbyClass "/Script/Engine.StaticMeshComponent"))
  (bind _outactors (Actor|GetAllActorsOfClass "/Game/ThirdPerson/Blueprints/BP_ThirdPersonCharacter.BP_ThirdPersonCharacter_C"))
  (Variables|Default|SetHolder (Utilities|Array|Get(acopy) _outactors))
  (Physics|SetSimulatePhysics (Variables|Default|GetMyMesh) true)
  (Physics|SetEnableGravity (Variables|Default|GetMyMesh) false))

(fn ConstructionScript)

(fn PickUp
  (params (Handle :type Physics%20Handle%20Component%20Object%20Reference) (Primiti%20component :type Primitive%20Component%20Object%20Reference))
  ;[0.09835 0.6771 0.6569] Sets the object where we have told it to, and notifies the object it is picked up
  (Physics|Components|PhysicsHandle|GrabComponentatLocationwithRotation Handle Primiti%20component "None" (Transformation|GetWorldLocation Primiti%20component) (Transformation|GetWorldRotation Primiti%20component))
  (Variables|Default|SetIsPicked true))

(fn Drop
  (params (Handle :type Physics%20Handle%20Component%20Object%20Reference))
  ;[0.09835 0.6771 0.6569] releseas the object and calls the throw function
  (Physics|Components|PhysicsHandle|ReleaseComponent Handle)
  (CallFunction|Throw))

(fn Throw
  (bind _mymesh (Variables|Default|GetMyMesh))
  ;[0.09835 0.6771 0.6569] Activates the gravity of the object
  (Physics|SetEnableGravity _mymesh true)
  ;[0.09835 0.6771 0.6569] Impulses the object where the player is looking at with the character and notifies the object it is not picked
  (Physics|AddImpulse _mymesh (* (Transformation|GetActorForwardVector (Variables|Default|GetHolder)) (Variables|Default|GetThrowForce)) "None" true)
  (Variables|Default|SetIsPicked false))