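; BP_RegeneationChamber is a regeneration chamber that restores the player's health to MaxLife on overlap.
; At BeginPlay it caches the health system of the first BP_ThirdPersonCharacter found.
; Any non-physics-simulating component entering the Box starts a loop calling AddHealth by Heal until life reaches MaxLife.
; The loop has no delay, so healing completes within the overlap event, and the overlapping actor's identity is unchecked.
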(event OnComponentBeginOverlap(Box)
  (params (OverlappedComponent :type Primitive%20Component%20Object%20Reference) (OtherActor :type Actor%20Object%20Reference) (OtherComp :type Primitive%20Component%20Object%20Reference) (OtherBodyIndex :type Integer) (bFromSweep :type Boolean) (SweepResult :type Hit%20Result%20Structure%20%28by%20ref%29))
  ;[1 1 1] Checks if the player has entered the chamber
  (if (not (Physics|IsSimulatingPhysics OtherComp "None"))
    ;[0.09835 0.6771 0.6569] It tells the player they are healing, calls the add health event and checks if the player is fully healed
    (bind _output_get (Variables|Default|SetHealing true))
    (while _output_get
      (Default|AddHealth (Variables|Default|GetPlayerSystem) (Variables|Default|GetHeal) false)
      (if (not (< (Variables|/Game/MoraBermejoSebastian/BP_HealthSystem.BP_HealthSystem_C|GetCurrentLife (Variables|Default|GetPlayerSystem)) (Variables|Default|GetMaxLife)))
        (Variables|Default|SetHealing false)))))

(event EventBeginPlay
  ;[1 1 1] Gets the reference to the health system of the player
  (bind _outactors (Actor|GetAllActorsOfClass "/Game/ThirdPerson/Blueprints/BP_ThirdPersonCharacter.BP_ThirdPersonCharacter_C"))
  (Variables|Default|SetPlayerSystem (Variables|/Game/ThirdPerson/Blueprints/BP_ThirdPersonCharacter.BP_ThirdPersonCharacter_C|GetBP_HealthSystem (Utilities|Array|Get(acopy) _outactors))))

(fn ConstructionScript)