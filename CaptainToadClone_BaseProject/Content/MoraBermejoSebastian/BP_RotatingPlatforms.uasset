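; Switchable rotating platform that turns 90 degrees over a set Duration when switched on.
; RotateOnce computes the target from the current world rotation and drives RotateTimeline, which lerps between rotations along the shortest path.
; With BehaviorA, switching off plays the timeline in reverse from its end toward the starting rotation.
; Otherwise switching off does nothing and each finished turn becomes the new starting rotation.
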(event EventBeginPlay
  ;[0.09835 0.6771 0.6569] Gets the original rotation of the platform
  (bind _output_get (Variables|Default|SetCurrentRotation (Transformation|GetWorldRotation (Variables|Default|GetScene))))
  (Variables|Default|SetTargetRoation _output_get)
  (Variables|Default|SetRotating false))

(event EventSwitchON
  ;[0.09835 0.6771 0.6569] Tells the platform to rotate according to its behavior
  (CallFunction|RotateOnce))

(event EventSwitchOFF
  ;[0.09835 0.6771 0.6569] Turns off the rotation
  (if (Variables|Default|GetBehaviorA)
    (CallFunction|StopRotation)))

(fn ConstructionScript)

(fn StopRotation
  (bind _rotatetimeline (Variables|Default|GetRotateTimeline))
  ;[0.09835 0.6771 0.6569] It stops the timeline, tells the platform it is not rotating and sets it back to its original rotation
  (Audio|Components|Audio|Stop _rotatetimeline)
  (Variables|Default|SetRotating false)
  (Components|Timeline|ReversefromEnd _rotatetimeline))

(fn RotateOnce
  (bind _rotatetimeline (Variables|Default|GetRotateTimeline))
  ;[0.09835 0.6771 0.6569] Makes the target rotation 90 degrees from the original
  (Variables|Default|SetTargetRoation (Math|Rotator|CombineRotators (Transformation|GetWorldRotation (Variables|Default|GetScene)) "0.000000,90.000000,0.000000"))
  ;[0.09835 0.6771 0.6569] Tells the timeline how to behave
  (Audio|Components|Audio|Stop _rotatetimeline)
  (Components|Timeline|SetLooping _rotatetimeline false)
  (Components|Timeline|SetPlayRate _rotatetimeline (/ 1.0 (Variables|Default|GetDuration)))
  (Components|Timeline|PlayfromStart _rotatetimeline))