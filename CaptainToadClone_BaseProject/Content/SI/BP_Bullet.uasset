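; BP_Bullet is a projectile that damages the player's health and destroys itself after ten seconds.
; It moves along local X each tick with sweep, adding Speed unscaled by delta time.
; On capsule overlap with any component not simulating physics, it removes Damage from the first BP_ThirdPersonCharacter's BPHealthSystem, cached at BeginPlay, then destroys itself, without checking that the player was hit.
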(event OnComponentBeginOverlap(Capsule)
  (params (OverlappedComponent :type Primitive%20Component%20Object%20Reference) (OtherActor :type Actor%20Object%20Reference) (OtherComp :type Primitive%20Component%20Object%20Reference) (OtherBodyIndex :type Integer) (bFromSweep :type Boolean) (SweepResult :type Hit%20Result%20Structure%20%28by%20ref%29))
  (Development|PrintString (Utilities|GetDisplayName OtherComp))
  (if (not (Physics|IsSimulatingPhysics OtherComp "None"))
    (Default|RemoveHealth (Variables|Default|GetPlayerSystem) (Variables|Default|GetDamage))
    (Actor|DestroyActor)))

(event EventBeginPlay
  (bind _outactors (Actor|GetAllActorsOfClass "/Game/ThirdPerson/Blueprints/BP_ThirdPersonCharacter.BP_ThirdPersonCharacter_C"))
  (Variables|Default|SetPlayerSystem (Variables|/Game/ThirdPerson/Blueprints/BP_ThirdPersonCharacter.BP_ThirdPersonCharacter_C|GetBP_HealthSystem (Utilities|Array|Get(acopy) _outactors))))

(event EventTick
  (params (DeltaSeconds :type Float%20%28single-precision%29))
  (Transformation|AddActorLocalOffset (Math|Vector|MakeVector (+ (Variables|Default|GetSpeed) (* (.x (Math|Vector|GetRightVector (Variables|Default|GetStaticMesh))) DeltaSeconds)) 0.0 0.0) true false)
  (Utilities|FlowControl|Delay 1e+01)
  (Actor|DestroyActor))

(fn ConstructionScript
  (|CallParentFunction))