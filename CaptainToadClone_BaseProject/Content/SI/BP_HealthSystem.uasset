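; BP_HealthSystem is a health component-style Blueprint that tracks current life against a maximum, starting full on BeginPlay.
; AddHealth and RemoveHealth clamp life between zero and the maximum, then broadcast healed or damaged events plus a general health-changed event.
; A separate Death function prints a death message and opens a given level by name; nothing here calls it automatically when life reaches zero.
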(event EventBeginPlay
  (Variables|Default|SetCurrentLife (Variables|Default|GetMaxLife)))

(fn AddHealth
  (params (Amount :type Float%20%28double-precision%29))
  (bind _output_get (Variables|Default|SetCurrentLife (Math|Float|Clamp(Float) (+ (Variables|Default|GetCurrentLife) Amount) 0.0 (Variables|Default|GetMaxLife))))
  (Default|CallOnHealthHealed Amount)
  (Default|CallOnHealthChanged _output_get))

(fn RemoveHealth
  (params (Amount :type Float%20%28double-precision%29))
  (bind _output_get (Variables|Default|SetCurrentLife (Math|Float|Clamp(Float) (- (Variables|Default|GetCurrentLife) Amount) 0.0 (Variables|Default|GetMaxLife))))
  (Default|CallOnHealthDamaged Amount)
  (Default|CallOnHealthChanged _output_get))

(fn Death
  (params (LevelName :type String))
  (Development|PrintString "YOU DIED" true true "(R=0.000000,G=0.660000,B=1.000000,A=1.000000)" 1e+01)
  (Game|OpenLevel(byName) (Utilities|String|StringToName LevelName)))