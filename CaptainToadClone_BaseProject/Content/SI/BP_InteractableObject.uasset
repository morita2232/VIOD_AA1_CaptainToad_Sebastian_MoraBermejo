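; BP_InteractableObject is a signal sender that switches a list of actors on or off.
; Encendido (on) and Apagado (off) loop over the Actores array and send SwitchONMessage or SwitchOFFMessage to each element implementing I_SignalReceiver.
; Non-implementers only trigger a debug print, and Apagado also prints on each call.
; Nothing in this Blueprint triggers either function, as the lone Encendido call in the EventGraph is unconnected.
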(fn ConstructionScript)

(fn Encendido
  (for _array_element (Variables|Default|GetActores)
    (if (Utilities|DoesObjectImplementInterface _array_element "/Game/SI/I_SignalReceiver.I_SignalReceiver_C")
      (Class|ISignalReceiver|SwitchON(Message) _array_element)
      (else
        (Development|PrintString "Pues no")))))

(fn Apagado
  (Development|PrintString "APAGADO")
  (for _array_element (Variables|Default|GetActores)
    (if (Utilities|DoesObjectImplementInterface _array_element "/Game/SI/I_SignalReceiver.I_SignalReceiver_C")
      (Class|ISignalReceiver|SwitchOFF(Message) _array_element)
      (else
        (Development|PrintString "Pues no")))))