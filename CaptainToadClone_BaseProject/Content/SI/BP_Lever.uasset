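; BP_Lever is an interactable lever that toggles between on and off calls and animates its skeletal mesh.
; On BeginPlay it caches the first BP_ThirdPersonCharacter found.
; INTERACT alternates Encendido and Apagado through a FlipFlop, setting the character's Onoff to true on both branches.
; UPDATE picks the toggle animation from that flag, so the interaction path always selects the toggle-off animation.
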(event Custom|INTERACT
  (Utilities|FlowControl|FlipFlop
    (:A
      (CallFunction|Encendido)
      (Variables|/Game/ThirdPerson/Blueprints/BP_ThirdPersonCharacter.BP_ThirdPersonCharacter_C|Seton/off (Variables|Default|GetCharacter) true))
    (:B
      (CallFunction|Apagado)
      (Variables|/Game/ThirdPerson/Blueprints/BP_ThirdPersonCharacter.BP_ThirdPersonCharacter_C|Seton/off (Variables|Default|GetCharacter) true)))
  (CallFunction|UPDATE))

(event Custom|UPDATE
  (if (Variables|/Game/ThirdPerson/Blueprints/BP_ThirdPersonCharacter.BP_ThirdPersonCharacter_C|Geton/off (Variables|Default|GetCharacter))
    (Components|Animation|PlayAnimation (Variables|Default|GetSkeletalMesh) "/Game/Assets/lever_Anim_toggle-off.lever_Anim_toggle-off" false)
    (else
      (Components|Animation|PlayAnimation (Variables|Default|GetSkeletalMesh) "/Game/Assets/lever_Anim_toggle-on.lever_Anim_toggle-on" false))))

(event EventBeginPlay
  (bind _outactors (Actor|GetAllActorsOfClass "/Game/ThirdPerson/Blueprints/BP_ThirdPersonCharacter.BP_ThirdPersonCharacter_C"))
  (Variables|Default|SetCharacter (Utilities|Array|Get(acopy) _outactors)))

(fn ConstructionScript
  (|CallParentFunction))