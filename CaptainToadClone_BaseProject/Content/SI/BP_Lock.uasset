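; BP_Lock is a lock actor that opens when the BP_Key actor is brought into its trigger box.
; On BeginPlay it caches the BP_Key found in the level with GetActorOfClass, so it responds to that one key instance only.
; When that key overlaps the Box, the lock fires Encendido, clears the key's IsPicked flag, and destroys both itself and the key.
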(event OnComponentBeginOverlap(Box)
  (params (OverlappedComponent :type Primitive%20Component%20Object%20Reference) (OtherActor :type Actor%20Object%20Reference) (OtherComp :type Primitive%20Component%20Object%20Reference) (OtherBodyIndex :type Integer) (bFromSweep :type Boolean) (SweepResult :type Hit%20Result%20Structure%20%28by%20ref%29))
  (if (== OtherActor (Variables|Default|GetKey))
    (CallFunction|Encendido)
    (Variables|/Game/SI/BP_PickableObject.BP_PickableObject_C|SetIsPicked (Variables|Default|GetKey) false)
    (Actor|DestroyActor)
    (Actor|DestroyActor OtherActor)))

(event EventBeginPlay
  (bind _returnvalue (Actor|GetActorOfClass "/Game/SI/BP_Key.BP_Key_C"))
  (Variables|Default|SetKey _returnvalue))

(fn ConstructionScript
  (|CallParentFunction))