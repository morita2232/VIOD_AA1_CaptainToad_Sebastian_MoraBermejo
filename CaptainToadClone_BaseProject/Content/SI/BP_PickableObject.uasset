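; BP_PickableObject is a physics object that can be picked up through a physics handle and is thrown when dropped.
; On BeginPlay it caches its static mesh and the first BP_ThirdPersonCharacter as holder, simulating physics with gravity off.
; PickUp grabs the passed component at its current transform.
; Drop releases it and calls Throw, which enables gravity and applies a velocity-change impulse along the holder's forward vector.
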(event EventBeginPlay
  (Variables|Default|SetMyMesh (Actor|GetComponentbyClass "/Script/Engine.StaticMeshComponent"))
  (bind _outactors (Actor|GetAllActorsOfClass "/Game/ThirdPerson/Blueprints/BP_ThirdPersonCharacter.BP_ThirdPersonCharacter_C"))
  (Variables|Default|SetHolder (Utilities|Array|Get(acopy) _outactors))
  (Physics|SetSimulatePhysics (Variables|Default|GetMyMesh) true)
  (Physics|SetEnableGravity (Variables|Default|GetMyMesh) false))

(fn ConstructionScript)

(fn PickUp
  (params (Handle :type Physics%20Handle%20Component%20Object%20Reference) (Primiti%20component :type Primitive%20Component%20Object%20Reference))
  (Development|PrintString "before hold")
  (Physics|Components|PhysicsHandle|GrabComponentatLocationwithRotation Handle Primiti%20component "None" (Transformation|GetWorldLocation Primiti%20component) (Transformation|GetWorldRotation Primiti%20component))
  (Development|PrintString "after hold")
  (Variables|Default|SetIsPicked true))

(fn Drop
  (params (Handle :type Physics%20Handle%20Component%20Object%20Reference))
  (Physics|Components|PhysicsHandle|ReleaseComponent Handle)
  (Development|PrintString "adeuuu")
  (CallFunction|Throw))

(fn Throw
  (bind _mymesh (Variables|Default|GetMyMesh))
  (Physics|SetEnableGravity _mymesh true)
  (Physics|AddImpulse _mymesh (* (Transformation|GetActorForwardVector (Variables|Default|GetHolder)) (Variables|Default|GetThrowForce)) "None" true)
  (Variables|Default|SetIsPicked false)
  (Development|PrintString "tirado"))