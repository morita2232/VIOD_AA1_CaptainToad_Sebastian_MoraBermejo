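; A rotating platform actor driven by SwitchON and SwitchOFF events, with two modes chosen by BehaviorA.
; With BehaviorA set, a looping timeline spins it in yaw at Speed until switched off, when it snaps back to its starting rotation.
; Otherwise, each SwitchON restarts the timeline to lerp a 90-degree step scaled to Duration, and SwitchOFF does nothing.
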(event EventBeginPlay
  (bind _output_get (Variables|Default|SetCurrentRotation (Transformation|GetWorldRotation (Variables|Default|GetScene))))
  (Variables|Default|SetTargetRoation _output_get)
  (Variables|Default|SetRotating false)
  (if (Variables|Default|GetBehaviorA)
    (Components|Timeline|SetLooping (Variables|Default|GetRotateTimeline) true)
    (else
      (Components|Timeline|SetLooping (Variables|Default|GetRotateTimeline) false))))

(event EventSwitchON
  (if (Variables|Default|GetBehaviorA)
    (CallFunction|StartRotation)
    (else
      (Development|PrintString (Utilities|String|ToString(Rotator) (Variables|Default|GetTargetRoation)))
      (CallFunction|RotateOnce)
      (Development|PrintString (Utilities|String|ToString(Rotator) (Variables|Default|GetTargetRoation))))))

(event EventSwitchOFF
  (if (Variables|Default|GetBehaviorA)
    (CallFunction|StopRotation)))

(fn ConstructionScript)

(fn StartRotation
  (if (not (Variables|Default|GetRotating))
    (Variables|Default|SetRotating true)
    (Audio|Components|Audio|Play (Variables|Default|GetRotateTimeline))))

(fn StopRotation
  (Audio|Components|Audio|Stop (Variables|Default|GetRotateTimeline))
  (Variables|Default|SetRotating false)
  (Transformation|SetWorldRotation (Variables|Default|GetScene) (Variables|Default|GetCurrentRotation) false false))

(fn RotateOnce
  (bind _rotatetimeline (Variables|Default|GetRotateTimeline))
  (Variables|Default|SetTargetRoation (Math|Rotator|CombineRotators (Transformation|GetWorldRotation (Variables|Default|GetScene)) "0.000000,90.000000,0.000000"))
  (Audio|Components|Audio|Stop _rotatetimeline)
  (Components|Timeline|SetLooping _rotatetimeline false)
  (Components|Timeline|SetPlayRate _rotatetimeline (/ 1.0 (Variables|Default|GetDuration)))
  (Components|Timeline|PlayfromStart _rotatetimeline))