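; BP_Spikes is a spike hazard that kills the player through the character's health system.
; On BeginPlay it caches the current level name and the BPHealthSystem of the first BP_ThirdPersonCharacter found.
; When any component not simulating physics overlaps its Box, it calls Death on that cached system with the level name, without checking that the player caused the overlap.
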(event OnComponentBeginOverlap(Box)
  (params (OverlappedComponent :type Primitive%20Component%20Object%20Reference) (OtherActor :type Actor%20Object%20Reference) (OtherComp :type Primitive%20Component%20Object%20Reference) (OtherBodyIndex :type Integer) (bFromSweep :type Boolean) (SweepResult :type Hit%20Result%20Structure%20%28by%20ref%29))
  (if (not (Physics|IsSimulatingPhysics OtherComp "None"))
    (Default|Death (Variables|Default|GetPlayerSystem) (Variables|Default|GetLevelName))))

(event EventBeginPlay
  (bind _returnvalue (Game|GetCurrentLevelName true))
  (Variables|Default|SetLevelName _returnvalue)
  (bind _outactors (Actor|GetAllActorsOfClass "/Game/ThirdPerson/Blueprints/BP_ThirdPersonCharacter.BP_ThirdPersonCharacter_C"))
  (Variables|Default|SetPlayerSystem (Variables|/Game/ThirdPerson/Blueprints/BP_ThirdPersonCharacter.BP_ThirdPersonCharacter_C|GetBP_HealthSystem (Utilities|Array|Get(acopy) _outactors))))

(fn ConstructionScript)